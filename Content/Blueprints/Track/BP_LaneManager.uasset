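; BP_LaneManager is a track actor that previews lane layout with debug drawing, and has no active runtime logic.
; Its construction script flushes persistent debug lines and loads the StandardLaneSegment class to read segment length and width from its defaults.
; For each entry in LanePositions, it draws a long-lived row of segment-sized boxes stepping along X, showing where lane segments would sit.
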(event EventBeginPlay)

(event Collision|EventActorBeginOverlap
  (params (OtherActor :type Actor%20Object%20Reference)))

(event EventTick
  (params (DeltaSeconds :type Float%20%28single-precision%29)))

(fn ConstructionScript
  (bind _standardlanesegment (Variables|Default|GetStandardLaneSegment))
  (bind _output (Utilities|ResolveSoftReference _standardlanesegment))
  (bind (_segmentspeed _segmentlength _segmentwidth) (Utilities|GetClassDefaults _output))
  (Rendering|Debug|FlushPersistentDebugLines)
  (Utilities|LoadClassAssetBlocking _standardlanesegment)
  (for _array_element (Variables|Default|GetLanePositions)
    (for _index (range 0 25)
      (Rendering|Debug|DrawDebugBox :Center (Math|Vector|MakeVector (+ (* _index _segmentlength) (.x _array_element)) (.y _array_element) (.z _array_element)) :Extent (Math|Vector|MakeVector (/ _segmentlength 2.0) (/ _segmentwidth 2.0) 1e+02) :Duration 9999.0 :Thickness 5.0))))