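; Player vehicle Blueprint that animates lane changes, jumps and side flips, and shows whether input is available.
; Timelines drive lane and jump movement from a stored origin, with play rates scaled by duration variables, calling completion functions when finished.
; Side changes quaternion-slerp the mesh to a pitch set by the side index.
; Tick swaps four planes between red locked and blue available dynamic materials based on input state.
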(event EventBeginPlay
  (bind _returnvalue (Rendering|Material|CreateDynamicMaterialInstance (Variables|Default|GetPlane) 0 "/Game/StarterContent/Materials/M_Basic_Wall.M_Basic_Wall" "None" :!class /Script/Engine.PrimitiveComponent))
  (Rendering|Material|SetVectorParameterValue _returnvalue "Color" "(R=1.000000,G=0.019096,B=0.000000,A=1.000000)" :!class /Script/Engine.MaterialInstanceDynamic)
  (bind _output_get (Variables|Default|SetMI_InputLocked _returnvalue))
  (Rendering|Material|SetMaterial (Variables|Default|GetPlane2) 0 _output_get)
  (Rendering|Material|SetMaterial (Variables|Default|GetPlane3) 0 _output_get)
  (Rendering|Material|SetMaterial (Variables|Default|GetPlane1) 0 _output_get)
  (bind _returnvalue_2 (Rendering|Material|CreateDynamicMaterialInstance (Variables|Default|GetPlane) 0 "/Game/StarterContent/Materials/M_Basic_Wall.M_Basic_Wall" "None" :!class /Script/Engine.PrimitiveComponent))
  (Rendering|Material|SetVectorParameterValue _returnvalue_2 "Color" "(R=0.014317,G=0.105290,B=1.000000,A=1.000000)" :!class /Script/Engine.MaterialInstanceDynamic)
  (bind _output_get_2 (Variables|Default|SetMI_InputAvailable _returnvalue_2))
  (Rendering|Material|SetMaterial (Variables|Default|GetPlane2) 0 _output_get_2)
  (Rendering|Material|SetMaterial (Variables|Default|GetPlane3) 0 _output_get_2)
  (Rendering|Material|SetMaterial (Variables|Default|GetPlane1) 0 _output_get_2))

(event EventJumpEvent
  (bind _returnvalue (Transformation|GetActorLocation))
  (Variables|Default|SetJumpOriginLocation (Transformation|GetActorLocation))
  (Components|Timeline|SetPlayRate (Variables|Default|GetTL_Jump) (/ 1.0 (Variables|Default|GetJumpHangTime)))
  (bind _jumpheightmod (Timeline|TL_Jump PlayFromStart)
    (:Update
      (Transformation|SetActorLocation (Math|Vector|MakeVector (.x _returnvalue) (.y _returnvalue) (+ (* _jumpheightmod (Variables|Default|GetJumpHeight)) (.z (Variables|Default|GetJumpOriginLocation)))) false false))
    (:Finished
      (Class|LaneVehicle|JumpEnded))))

(event EventTick
  (params (DeltaSeconds :type Float%20%28single-precision%29))
  (bind _mi_inputlocked (Variables|Default|GetMI_InputLocked))
  (bind _mi_inputavailable (Variables|Default|GetMI_InputAvailable))
  (switch Utilities|FlowControl|Switch|SwitchonEVehicleInputState (Variables|Default|GetVehicleInputState)
    (:EVIS_Available
      (Rendering|Material|SetMaterial (Variables|Default|GetPlane1) 0 _mi_inputavailable)
      (Rendering|Material|SetMaterial (Variables|Default|GetPlane2) 0 _mi_inputavailable)
      (Rendering|Material|SetMaterial (Variables|Default|GetPlane3) 0 _mi_inputavailable)
      (Rendering|Material|SetMaterial (Variables|Default|GetPlane) 0 _mi_inputavailable))
    (:EVIS_Processing
      (Rendering|Material|SetMaterial (Variables|Default|GetPlane1) 0 _mi_inputlocked)
      (Rendering|Material|SetMaterial (Variables|Default|GetPlane2) 0 _mi_inputlocked)
      (Rendering|Material|SetMaterial (Variables|Default|GetPlane3) 0 _mi_inputlocked)
      (Rendering|Material|SetMaterial (Variables|Default|GetPlane) 0 _mi_inputlocked))))

(event EventSideChanged
  (Variables|Default|SetOriginalQuat (Math|Conversions|ToQuaternion(Rotator) (Variables|/Script/Engine.SceneComponent|GetRelativeRotation (Variables|Default|GetVehicleMesh))))
  (bind _newtrack_0 (Timeline|TL_SideChanged PlayFromStart)
    (:Update
      (Transformation|SetRelativeRotation (Variables|Default|GetVehicleMesh) (Class|KismetMathLibrary|QuatRotator (Class|KismetMathLibrary|QuatSlerp (Variables|Default|GetOriginalQuat) (Math|Conversions|ToQuaternion(Rotator) (Math|Rotator|MakeRotator 0.0 (* (Variables|Default|GetSideUpIndex) -9e+01) -9e+01)) _newtrack_0)) false false))))

(event EventLaneChanged
  (params (NewVehicleLocation :type Vector :default "0, 0, 0"))
  (bind _returnvalue (Transformation|GetActorLocation))
  (Variables|Default|SetLaneOriginLoc _returnvalue)
  (Variables|Default|SetLaneTravelDistance (- NewVehicleLocation _returnvalue))
  (Components|Timeline|SetPlayRate (Variables|Default|GetTL_LaneChange) (/ 1.0 (Variables|Default|GetLaneChangeTime)))
  (bind _newtrack_0 (Timeline|TL_LaneChange PlayFromStart)
    (:Update
      (Transformation|SetActorLocation (+ (Variables|Default|GetLaneOriginLoc) (* _newtrack_0 (Variables|Default|GetLaneTravelDistance))) false false))
    (:Finished
      (Class|LaneVehicle|LaneChangeComplete))))

(fn ConstructionScript)